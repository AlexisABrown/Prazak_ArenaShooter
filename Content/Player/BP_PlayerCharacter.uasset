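; BP_PlayerCharacter is the player character Blueprint, handling basic walking, mouse look and jumping.
; MoveForward and MoveLeft axes feed movement input along the full control rotation's forward and right vectors, so positive MoveLeft values point right.
; Turn and LookUp drive controller yaw and pitch, while Jump press and release start and stop jumping.
; BeginPlay, overlap, Tick and the construction script contain no logic.
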(event `InputAxis|MoveForward`
  (params (AxisValue :type "Float (single-precision)"))
  ;[1 1 1] Player Movement
  (`self.AddMovementInput` (`KismetMathLibrary.GetForwardVector` (`self.GetControlRotation`)) AxisValue))

(event `InputAxis|MoveLeft`
  (params (AxisValue :type "Float (single-precision)"))
  ;[1 1 1] Player Movement
  (`self.AddMovementInput` (`KismetMathLibrary.GetRightVector` (`self.GetControlRotation`)) AxisValue))

(event `InputAxis|Turn`
  (params (AxisValue :type "Float (single-precision)"))
  ;[1 1 1] Allows Player to look around using mouse
  (`self.AddControllerYawInput` AxisValue))

(event `InputAction|Jump`
  (params (Key :type "Key Structure"))
  ;[1 1 1] Player Jump
  (:`Pressed`
    (`self.Jump`))
  (:`Released`
    (`self.StopJumping`)))

(event `InputAxis|LookUp`
  (params (AxisValue :type "Float (single-precision)"))
  ;[1 1 1] Allows Player to look around using mouse
  (`self.AddControllerPitchInput` AxisValue))

(fn `UserConstructionScript`)