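; BP_EnemyProjectileBase is a projectile that deals fixed damage to characters it overlaps and expires a few seconds after spawning.
; Its collision overlap casts the other actor to BP_AICharacter, then BP_PlayerCharacter, ignoring anything else, so AI characters can be hit as well as the player.
; Each branch uses a DoOnce to apply damage with the projectile's owner as causer, then destroys the projectile.
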(event `self.ReceiveBeginPlay`
  ;[1 1 1] Destroy projectile after firing
  (`KismetSystemLibrary.Delay` 3.0)
  (`self.K2_DestroyActor`))

(event `self.ProjectileCollision.OnComponentBeginOverlap`
  (params (OverlappedComponent :type "PrimitiveComponent Object Reference") (OtherActor :type "Actor Object Reference") (OtherComp :type "PrimitiveComponent Object Reference") (OtherBodyIndex :type Integer) (bFromSweep :type Boolean) (SweepResult :type "HitResult Structure (by ref)"))
  (bind _returnvalue (`self.GetOwner`))
  (bind _asbp_aicharacter (cast `/Game/AI/BP_AICharacter` OtherActor)
    (:`then`
      (if true
        (`/Engine/EditorBlueprintResources/StandardMacros.DoOnce` false
          (:`Completed`
            (`GameplayStatics.ApplyDamage` _asbp_aicharacter 10.0 null _returnvalue)
            (`self.K2_DestroyActor` :!label _label)))))
    (:`CastFailed`
      (bind _asbp_player_character (cast `/Game/Player/BP_PlayerCharacter` OtherActor))
      (`/Engine/EditorBlueprintResources/StandardMacros.DoOnce` false
        (:`Completed`
          (`GameplayStatics.ApplyDamage` _asbp_player_character 10.0 null _returnvalue)
          (goto _label))))))

(fn `UserConstructionScript`)